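; Actor component that gives its owning Character flight, switching movement between Flying and Falling on start and stop.
; On BeginPlay it caches character references and applies hover speed, acceleration, rotation and braking settings.
; In networked play the local change goes through server and multicast events, which skip the locally controlled character.
; Each tick it updates speed and movement-input state, and derives a smoothed Lean vector from yaw and pitch rates of velocity rotation.
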(event `self.ReceiveBeginPlay`
  (bind _returnvalue (`Actor.GetComponentByClass` (`self.Character`) "/Script/Engine.CameraComponent"))
  (bind _returnvalue_2 (`Actor.GetComponentByClass` (`self.Character`) "/Script/Engine.SpringArmComponent"))
  (bind _ascharacter (cast `Character` (`self.GetOwner`)))
  (set `self.Character` _ascharacter)
  (set `self.Character Movement` (`Character.CharacterMovement` _ascharacter))
  (set `self.AnimInstance` (`SkeletalMeshComponent.GetAnimInstance` (`Character.Mesh` (`self.Character`))))
  (`/Engine/EditorBlueprintResources/StandardMacros.IsValid` _returnvalue_2
    (:`Is Valid`
      (set `self.Spring Arm` _returnvalue_2))
    (:`Is Not Valid`
      _))
  (`/Engine/EditorBlueprintResources/StandardMacros.IsValid` _returnvalue
    (:`Is Valid`
      (set `self.Camera` _returnvalue)
      (`self.SetFlightMovementParam`))))

(event `SRV_ Set Has Movement Input`
  (`self.SetHasMovementInput` (`self.HasMovementInput`)))

(event `self.ReceiveTick`
  (params (DeltaSeconds :type "Float (single-precision)"))
  (bind _returnvalue (`GameplayStatics.GetWorldDeltaSeconds`))
  (bind _last_velocity_rotation (`self.Last Velocity Rotation`))
  (bind (_lean_x _lean_y) (`KismetMathLibrary.BreakVector2D` (`self.Lean`)))
  (bind (_returnvalue_roll _returnvalue_pitch _returnvalue_yaw) (`KismetMathLibrary.BreakRotator` (`KismetMathLibrary.NormalizedDeltaRotator` _last_velocity_rotation (`self.Previous Velocity Rotation`))))
  (bind (_returnvalue_roll_2 _returnvalue_pitch_2 _returnvalue_yaw_2) (`KismetMathLibrary.BreakRotator` (`Actor.K2_GetActorRotation` (`self.Character`))))
  (bind (_returnvalue_roll_3 _returnvalue_pitch_3) (`KismetMathLibrary.BreakRotator` (`KismetMathLibrary.Conv_VectorToRotator` (`Actor.GetVelocity` (`self.Character`)))))
  (`|ExecutionSequence`
    (:`then_0`
      (if (!= (`KismetMathLibrary.VSize` (`Actor.GetVelocity` (`self.Character`))) 0.0)
        (set `self.Last Velocity Rotation` (`KismetMathLibrary.MakeRotator` _returnvalue_roll_2 _returnvalue_pitch_3 _returnvalue_yaw_2))
        (set `self.Current Speed` (`KismetMathLibrary.VSize` (`Actor.GetVelocity` (`self.Character`))))))
    (:`then_1`
      (`self.Is Networked`
        (:`True`
          (`self.SRV_ Set Has Movement Input`))
        (:`False`
          (`self.SetHasMovementInput` (`self.HasMovementInput`)))))
    (:`then_2`
      (bind _output_get (set `self.Yaw Velocity Difference` (/ _returnvalue_yaw (`GameplayStatics.GetWorldDeltaSeconds`))))
      (bind _output_get_2 (set `self.Pitch Velocity Difference` (/ _returnvalue_pitch (`GameplayStatics.GetWorldDeltaSeconds`))))
      (set `self.Previous Velocity Rotation` _last_velocity_rotation)
      (set `self.Lean` (`KismetMathLibrary.MakeVector2D` (`KismetMathLibrary.FInterpTo` _lean_x (`KismetMathLibrary.MapRangeClamped` _output_get -180.0 180.0 -1.0 1.0) _returnvalue 5.0) (`KismetMathLibrary.FInterpTo` _lean_y (`KismetMathLibrary.MapRangeClamped` _output_get_2 -180.0 180.0 -1.0 1.0) _returnvalue 15.0))))))

(event `Start Fly`
  ;[1 1 1] Start/Stop Flight Event
  (`self.SetIsFlying` true)
  (`self.Is Networked`
    (:`True`
      (`self.SetMovementMode( SERVER )` true))))

(event `Stop Fly`
  ;[1 1 1] Start/Stop Flight Event
  (`self.SetIsFlying` false)
  (`self.Is Networked`
    (:`True`
      (`self.SetMovementMode( SERVER )` false))))

(event `SetMovementMode( SERVER )`
  (params (IsFlying :type Boolean))
  ;[1 1 1] Set"Movement Mode" replicated
  (`self.SetMovementMode( MULTICAST )` IsFlying))

(event `SetMovementMode( MULTICAST )`
  (params (IsFlying :type Boolean))
  ;[1 1 1] Set"Movement Mode" replicated
  (`self.IsLocallyControlled`
    (:`False`
      (`self.SetIsFlying` IsFlying))))

(fn `GetLean`
  (returns (Lean :type "Vector2D Structure"))
  (return (`self.Lean`)))

(fn `SetFlightMovementParam`
  (set `CharacterMovementComponent.MaxFlySpeed` (`self.Hover Fly Speed`) (`self.Character Movement`))
  (set `CharacterMovementComponent.MaxAcceleration` (`self.Hover Acceleration`) (`self.Character Movement`))
  (set `CharacterMovementComponent.RotationRate` (`self.Hover Rotation Rate`) (`self.Character Movement`))
  (set `CharacterMovementComponent.BrakingDecelerationFlying` (`self.Flight Breaking Deceleration`) (`self.Character Movement`)))

(fn `SetHasMovementInput`
  (params (`Has Movement Input` :type Boolean))
  (set `self.Has Movement Input` `Has Movement Input`))

(fn `SetIsFlying`
  (params (IsFlying :type Boolean))
  (bind _output_get (set `self.IsFlying` IsFlying))
  (if _output_get
    (`self.SetMovementMode` "MOVE_Flying")
    (else
      (`self.SetMovementMode` "MOVE_Falling"))))

(fn `SetMovementMode`
  (params (MovementMode :type "EMovementMode Enum" :default "MOVE_None"))
  (bind _character_movement (`self.Character Movement`))
  (`/Engine/EditorBlueprintResources/StandardMacros.IsValid` _character_movement
    (:`Is Valid`
      (`CharacterMovementComponent.SetMovementMode` _character_movement MovementMode 0))))